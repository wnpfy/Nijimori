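; BP_Player is a player pawn with axis-driven movement and mouse look, viewed through a lagging camera.
; Movement follows control yaw only, while look input is scaled by MouseStrength.
; On BeginPlay it spawns a separate CameraActor at its Camera component, applies the FOV and makes it the view target.
; Each tick that actor interpolates toward the Camera component's transform at LagSpeed, smoothing the view.
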(event EventBeginPlay
  (bind _returnvalue (Game|SpawnActorfromClass "/Script/Engine.CameraActor" (Transformation|GetWorldTransform (Variables|Default|GetCamera)) "Undefined" "MultiplyWithRoot" 0 0))
  (bind _output_get (Variables|Default|Setplayer%20camera _returnvalue))
  (Camera|SetFieldOfView (Variables|/Script/Engine.CameraActor|GetCameraComponent _output_get) (Variables|Default|GetFOV))
  (Class|CameraComponent|SetConstraintAspectRatio (Variables|/Script/Engine.CameraActor|GetCameraComponent _output_get) false)
  (Game|Player|SetViewTargetwithBlend (Game|GetPlayerController 0) (Variables|Default|Getplayer%20camera) 0.0 "VTBlend_Linear" 0.0 false))

(event EventTick
  (params (DeltaSeconds :type Float%20%28single-precision%29))
  (Transformation|SetActorTransform (Variables|Default|Getplayer%20camera) (Class|KismetMathLibrary|TInterpto (Transformation|GetActorTransform (Variables|Default|Getplayer%20camera)) (Transformation|GetWorldTransform (Variables|Default|GetCamera)) DeltaSeconds (Variables|Default|GetLagSpeed))))

(event Input|AxisEvents|InputAxisLookUp
  (params (AxisValue :type Float%20%28single-precision%29))
  (Pawn|Input|AddControllerPitchInput (* AxisValue (Variables|Default|GetMouseStrength))))

(event Input|AxisEvents|InputAxisLookRight
  (params (AxisValue :type Float%20%28single-precision%29))
  (Pawn|Input|AddControllerYawInput (* (Variables|Default|GetMouseStrength) AxisValue)))

(event Input|AxisEvents|InputAxisMoveforward
  (params (AxisValue :type Float%20%28single-precision%29))
  (Pawn|Input|AddMovementInput (Math|Vector|GetForwardVector (Math|Rotator|MakeRotator 0.0 0.0 (.Yaw (Math|Rotator|BreakRotator (Pawn|GetControlRotation :!class /Script/Engine.Pawn))))) AxisValue false))

(event Input|AxisEvents|InputAxisMoveRight
  (params (AxisValue :type Float%20%28single-precision%29))
  (Pawn|Input|AddMovementInput (Math|Vector|GetRightVector (Math|Rotator|MakeRotator 0.0 0.0 (.Yaw (Math|Rotator|BreakRotator (Pawn|GetControlRotation :!class /Script/Engine.Pawn))))) AxisValue false))

(fn ConstructionScript)